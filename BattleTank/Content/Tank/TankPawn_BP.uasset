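; Player-controllable tank pawn that wires up the tank's aiming and movement components and binds input for camera, driving and firing.
; On BeginPlay it hands the turret and barrel to TankAiming and both tracks to TankMovement.
; Forward and Right axes pass movement intent to TankMovement, and the Fire action calls Fire.
; Camera axes yaw the azimuth gimbal and pitch the spring arm separately, scaled by delta time.
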(event `self.ReceiveBeginPlay`
  (`KismetSystemLibrary.PrintString` "DONKEY: Tank BP BeginPlay!")
  (`TankAimingComponent.Initialise` (`self.TankAiming`) (`self.Turret`) (`self.Barrel`))
  (`TankMovementComponent.Initialise` (`self.TankMovement`) (`self.Left Track`) (`self.Right Track`)))

(event `InputAxis|AimAzimuth`
  (params (AxisValue :type "Float (single-precision)"))
  ;[1 1 1] Camera Input Binding
  (`SceneComponent.K2_AddLocalRotation` (`self.Azimuth Gimbal`) (`KismetMathLibrary.MakeRotator` 0.0 0.0 (* AxisValue (`GameplayStatics.GetWorldDeltaSeconds`) 100.0)) false false))

(event `InputAxis|Forward`
  (params (AxisValue :type "Float (single-precision)"))
  ;[1 1 1] Movement
  (`TankMovementComponent.IntendMoveForward` (`self.TankMovement`) AxisValue))

(event `InputAxis|Right`
  (params (AxisValue :type "Float (single-precision)"))
  ;[1 1 1] Movement
  (`TankMovementComponent.IntendTurnRight` (`self.TankMovement`) AxisValue))

(event `InputAxis|AimElevation`
  (params (AxisValue :type "Float (single-precision)"))
  ;[1 1 1] Camera Input Binding
  (`SceneComponent.K2_AddLocalRotation` (`self.SpringArm`) (`KismetMathLibrary.MakeRotator` 0.0 (* AxisValue (`GameplayStatics.GetWorldDeltaSeconds`) 100.0)) false false))

(event `InputAction|Fire`
  (params (Key :type "Key Structure" :default "AnyKey"))
  ;[1 1 1] Fire
  (:`Pressed`
    (`self.Fire`)))

(fn `UserConstructionScript`
  (`KismetSystemLibrary.PrintString` "DONKEY: Tank BP Constructor!"))